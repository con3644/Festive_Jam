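; LightsBP is a Christmas lights actor that pulses colored lights over time.
; Tick accumulates elapsed time and feeds an offset sine wave into the lights mesh's LightTime material parameter and, scaled by LightIntensity, into twelve light components.
; Yellow and green lights receive the negated value of red and blue, so the two color groups alternate.
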(event `self.ReceiveTick`
  (params (DeltaSeconds :type "Float (single-precision)"))
  (bind _output_get (set `self.Time Elapsed` (+ DeltaSeconds (`self.Time Elapsed`))))
  (bind _returnvalue (+ (`KismetMathLibrary.Sin` _output_get) 0.5))
  (`MeshComponent.SetScalarParameterValueOnMaterials` (`self.ChristmasLights`) "LightTime" _returnvalue)
  (bind _returnvalue_2 (* _returnvalue (`self.Light Intensity`)))
  (`LightComponent.SetIntensity` (`self.RedLight1`) _returnvalue_2)
  (`LightComponent.SetIntensity` (`self.RedLight2`) _returnvalue_2)
  (`LightComponent.SetIntensity` (`self.RedLight3`) _returnvalue_2)
  (`LightComponent.SetIntensity` (`self.BlueLight3`) _returnvalue_2)
  (`LightComponent.SetIntensity` (`self.BlueLight1`) _returnvalue_2)
  (`LightComponent.SetIntensity` (`self.BlueLight2`) _returnvalue_2)
  (bind _returnvalue_3 (* _returnvalue_2 -1.0))
  (`LightComponent.SetIntensity` (`self.YellowLight3`) _returnvalue_3)
  (`LightComponent.SetIntensity` (`self.YellowLight1`) _returnvalue_3)
  (`LightComponent.SetIntensity` (`self.YellowLight2`) _returnvalue_3)
  (`LightComponent.SetIntensity` (`self.GreenLight2`) _returnvalue_3)
  (`LightComponent.SetIntensity` (`self.GreenLight3`) _returnvalue_3)
  (`LightComponent.SetIntensity` (`self.GreenLight1`) _returnvalue_3))

(fn `UserConstructionScript`)