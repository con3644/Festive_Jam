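; TorchBP is a torch Blueprint that makes its PointLight flicker.
; Each Tick accumulates elapsed time and feeds it, times a newly randomized frequency, into a sine wave.
; The sine is clamped to a narrow band just below full brightness and scales LightIntensity to set the light's intensity.
; Re-rolling the frequency every frame makes the flicker erratic rather than periodic.
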(event `self.ReceiveTick`
  (params (DeltaSeconds :type "Float (single-precision)"))
  (bind _output_get (set `self.TimeElapsed` (+ DeltaSeconds (`self.TimeElapsed`))))
  (`LightComponent.SetIntensity` (`self.PointLight`) (* (`KismetMathLibrary.FClamp` (`KismetMathLibrary.Sin` (* _output_get (`KismetMathLibrary.RandomFloatInRange` 5.0 50.0))) 0.8) (`self.Light Intensity`))))

(fn `UserConstructionScript`)